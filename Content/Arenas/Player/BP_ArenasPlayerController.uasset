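; Arenas player controller that displays floating combat text for damage, gold and experience.
; On BeginPlay it spawns a BP_CombatText actor and initialises it with itself as parent and a vertical offset.
; ShowCombatText switches on text type to activate that actor at the hit location, overriding text, colours or icons for most types.
; Player-damaged text uses its preset style without overrides.
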(event `self.ReceiveBeginPlay`
  (bind _returnvalue (`|SpawnActorFromClass` "/Game/DynamicCombatText/Blueprints/BP_CombatText.BP_CombatText_C" (`KismetMathLibrary.MakeTransform` (0.0 0.0 0.0)) "Undefined" "OverrideRootScale" null null))
  (bind _output_get (set `self.CombatText` _returnvalue))
  (`/Game/DynamicCombatText/Blueprints/BP_CombatText.Initialise` _output_get self (0.0 0.0 175.0)))

(event `self.BP_ShowCombatText`
  (params (ValueNumber :type "Float (single-precision)") (TextType :type "EArenasComboTextType Enum" :default "Normal") (HitLocation :type "Vector Structure (by ref)"))
  (`self.CombatText`
    (:`then`
      (switch `EArenasComboTextType` TextType
        (:`Normal`
          ;[1 1 1] Critical Hit Damage
          (`/Game/DynamicCombatText/Blueprints/BP_CombatText.ActivateText_WithOverrides` (`self.CombatText`) "NewEnumerator14" 0.0 true HitLocation true (`KismetTextLibrary.Conv_DoubleToText` ValueNumber "HalfToEven" false true 1 324 0 0) true (struct :`R` 1.0 :`G` 0.336727 :`A` 1.0) false null true (struct :`R` 0.037241 :`G` 0.065068 :`B` 0.094792 :`A` 1.0) false (struct :`A` 1.0)))
        (:`Gold`
          ;[1 1 1] Gold
          (`/Game/DynamicCombatText/Blueprints/BP_CombatText.ActivateText_WithOverrides` (`self.CombatText`) "NewEnumerator23" ValueNumber true HitLocation true "Gold" true (struct :`R` 0.947307 :`G` 0.658375 :`B` 0.082283 :`A` 1.0) true "/Game/Arenas/Texture/gold_small.gold_small" false (struct :`A` 1.0) false (struct :`A` 1.0)))
        (:`Experience`
          ;[1 1 1] Normal damage
          (`/Game/DynamicCombatText/Blueprints/BP_CombatText.ActivateText_WithOverrides` (`self.CombatText`) "NewEnumerator23" ValueNumber true HitLocation true "EXP" true (struct :`R` 1.0 :`G` 1.0 :`B` 1.0 :`A` 1.0) true null false (struct :`A` 1.0) false (struct :`A` 1.0)))
        (:`Damaged`
          ;[1 1 1] Player Hit Damage
          (`/Game/DynamicCombatText/Blueprints/BP_CombatText.ActivateText` (`self.CombatText`) "NewEnumerator24" ValueNumber true HitLocation))
        (:`MagicDamaged`
          (`/Game/DynamicCombatText/Blueprints/BP_CombatText.ActivateText_WithOverrides` (`self.CombatText`) "NewEnumerator14" 0.0 true HitLocation true (`KismetTextLibrary.Conv_DoubleToText` ValueNumber "HalfToEven" false true 1 324 0 0) true (struct :`R` 0.026623 :`G` 0.569862 :`B` 1.0 :`A` 1.0) false null true (struct :`R` 0.037241 :`G` 0.065068 :`B` 0.094792 :`A` 1.0) false (struct :`A` 1.0)))))
    (:`else`)))

(fn `UserConstructionScript`)