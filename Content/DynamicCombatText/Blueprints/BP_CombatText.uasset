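; Actor that displays floating combat text for an owning actor using a pool of Widget_CombatText widget components created at BeginPlay.
; ActivateText picks an inactive widget, moves it to the owner plus offset or a custom location, and activates it with style properties looked up by text type.
; An override variant can replace the text, icon and colors.
; Initialise optionally attaches to the owner and starts a randomized looping timer for self-destruction once the owner is invalid.
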(event `self.ReceiveBeginPlay`
  ;[1 1 1] Create the required number of UCT widgets.
  ; Set self as a property on the widget so it can access this actor's variables.
  (for _ (range (`self.NumWidgetsPerActor`))
    (bind _returnvalue (`AddComponent|NODE_AddWidgetComponent-1` :`RelativeTransform` (`self.GetTransform`)))
    (`KismetArrayLibrary.Array_Add` (`self.WidgetComponents`) _returnvalue)
    (`ActorComponent.SetComponentTickEnabled` _returnvalue false)
    (`PrimitiveComponent.SetCollisionEnabled` _returnvalue "NoCollision")
    (bind _aswidget_combat_text (cast `/Game/DynamicCombatText/Blueprints/Widget_CombatText` (`WidgetComponent.GetUserWidgetObject` _returnvalue)))
    (set `/Game/DynamicCombatText/Blueprints/Widget_CombatText.ParentActor` self _aswidget_combat_text)
    (set `/Game/DynamicCombatText/Blueprints/Widget_CombatText.ParentWidgetComponent` _returnvalue _aswidget_combat_text)))

(fn `ActivateText`
  (params (Type :type "/Game/DynamicCombatText/Blueprints/ENUM_TextTypes Enum" :default "NewEnumerator0") (Value :type "Float (double-precision)") (CustomLocation :type Boolean) (WorldLocation :type "Vector Structure"))
  (locals (ChosenWidgetLocal :type "/Game/DynamicCombatText/Blueprints/Widget_CombatText Object Reference"))
  (bind _output (`|GetArrayItem` (`self.WidgetComponents`) (`self.FreeWidgetIndex`)))
  ;[1 1 1] Find the next free widget and activate it. Slightly different logic depending on whether to use a custom location.
  (bind _output_get (set `local.ChosenWidgetLocal` (`self.GetNextFreeWidget`)))
  (`/Engine/EditorBlueprintResources/StandardMacros.IsValid` _output_get
    (:`Is Valid`
      (if CustomLocation
        (`SceneComponent.K2_SetWorldLocation` _output WorldLocation false true)
        (else
          (`SceneComponent.K2_SetWorldLocation` _output (+ (`self.K2_GetActorLocation` (`self.ParentActor`)) (`self.StartingOffset`)) false true)))
      (`/Game/DynamicCombatText/Blueprints/Widget_CombatText.Activate` (`local.ChosenWidgetLocal`) (`self.FindProperties` Type) Value (`self.DecimalPrecision`)))))

(fn `ActivateText_WithOverrides`
  (params (Type :type "/Game/DynamicCombatText/Blueprints/ENUM_TextTypes Enum" :default "NewEnumerator0") (Value :type "Float (double-precision)") (CustomLocation :type Boolean) (WorldLocation :type "Vector Structure") (OverrideText :type Boolean) (Text :type Text) (OverrideColor :type Boolean) (TextColor :type "LinearColor Structure") (OverrideIcon :type Boolean) (Icon :type "Texture2D Object Reference") (OverrideOutlineColor :type Boolean) (OutlineColor :type "LinearColor Structure" :default (struct :`A` 1.0)) (OverrideShadowColor :type Boolean) (ShadowColor :type "LinearColor Structure" :default (struct :`A` 1.0)))
  (locals (ChosenWidgetLocal :type "/Game/DynamicCombatText/Blueprints/Widget_CombatText Object Reference") (FoundProperties :type "/Game/DynamicCombatText/Blueprints/STRUCT_TextTypeProperties Structure"))
  (bind _output (`|GetArrayItem` (`self.WidgetComponents`) (`self.FreeWidgetIndex`)))
  ;[1 1 1] Find the next free widget and activate it. Slightly different logic depending on whether to use a custom location.
  ; This version of the function allows overrides to several values.
  (bind _output_get (set `local.ChosenWidgetLocal` (`self.GetNextFreeWidget`)))
  (`/Engine/EditorBlueprintResources/StandardMacros.IsValid` _output_get
    (:`Is Valid`
      (`|ExecutionSequence`
        (:`then_0`
          (if CustomLocation
            (`SceneComponent.K2_SetWorldLocation` _output WorldLocation false true)
            (else
              (`SceneComponent.K2_SetWorldLocation` _output (+ (`self.K2_GetActorLocation` (`self.ParentActor`)) (`self.StartingOffset`)) false true)))
          (set `local.FoundProperties` (`self.FindProperties` Type))
          (`|ExecutionSequence`
            (:`then_0`
              (if OverrideText
                (setmembers `/Game/DynamicCombatText/Blueprints/STRUCT_TextTypeProperties` :`StructRef` (`local.FoundProperties`) :`Optional Message` Text)))
            (:`then_1`
              (if OverrideColor
                (setmembers `/Game/DynamicCombatText/Blueprints/STRUCT_TextTypeProperties` :`StructRef` (`local.FoundProperties`) :`Text Color` TextColor)))
            (:`then_2`
              (if OverrideIcon
                (setmembers `/Game/DynamicCombatText/Blueprints/STRUCT_TextTypeProperties` :`StructRef` (`local.FoundProperties`) :`Optional Icon` Icon)))))
        (:`then_1`
          (`|ExecutionSequence`
            (:`then_0`
              (if OverrideOutlineColor
                (setmembers `/Game/DynamicCombatText/Blueprints/STRUCT_TextTypeProperties` :`StructRef` (`local.FoundProperties`) :`Outline Color` OutlineColor)))
            (:`then_1`
              (if OverrideShadowColor
                (setmembers `/Game/DynamicCombatText/Blueprints/STRUCT_TextTypeProperties` :`StructRef` (`local.FoundProperties`) :`Shadow Color` ShadowColor)))))
        (:`then_2`
          (`/Game/DynamicCombatText/Blueprints/Widget_CombatText.Activate` (`local.ChosenWidgetLocal`) (`local.FoundProperties`) Value (`self.DecimalPrecision`)))))))

(fn `DestroyIfOwnerInvalid`
  ;[1 1 1] Destroy self if owner is invalid, for example if the parent is an enemy and it's just been removed from the game.
  (`/Engine/EditorBlueprintResources/StandardMacros.IsValid` (`self.ParentActor`)
    (:`Is Not Valid`
      (`self.K2_DestroyActor`))))

(fn `FindProperties`
  (params (Identifier :type "/Game/DynamicCombatText/Blueprints/ENUM_TextTypes Enum" :default "NewEnumerator0"))
  (returns (Index :type "/Game/DynamicCombatText/Blueprints/STRUCT_TextTypeProperties Structure"))
  (locals (ReturnProperties :type "/Game/DynamicCombatText/Blueprints/STRUCT_TextTypeProperties Structure"))
  ;[1 1 1] Return the set of properties associated with the Text Type.
  (for _array_element (`self.TextTypes`)
    (if (`|EnumEquality` (`.TextTypeIdentifier_75_BC786AAB4DF969DB54F88BB48D1A255E` (break `/Game/DynamicCombatText/Blueprints/STRUCT_TextTypeProperties` _array_element)) Identifier)
      (set `local.ReturnProperties` _array_element)
      (break)))
  (return (`local.ReturnProperties`)))

(fn `GetNextFreeWidget`
  (returns (Widget :type "/Game/DynamicCombatText/Blueprints/Widget_CombatText Object Reference"))
  (locals (FreeWidget :type "/Game/DynamicCombatText/Blueprints/Widget_CombatText Object Reference"))
  ;[1 1 1] Find the next free widget that isn't currently already on screen.
  (for (_array_element _array_index) (`self.WidgetComponents`)
    (bind _aswidget_combat_text (cast `/Game/DynamicCombatText/Blueprints/Widget_CombatText` (`WidgetComponent.GetUserWidgetObject` _array_element)))
    (if (not (`/Game/DynamicCombatText/Blueprints/Widget_CombatText.IsActive` _aswidget_combat_text))
      (set `self.FreeWidgetIndex` _array_index)
      (set `local.FreeWidget` _aswidget_combat_text)
      (break)))
  (return (`local.FreeWidget`)))

(fn `Initialise`
  (params (Parent :type "Actor Object Reference") (Offset :type "Vector Structure"))
  ;[1 1 1] Initialise variables
  (set `self.ParentActor` Parent)
  (set `self.StartingOffset` Offset)
  ;[1 1 1] Attach self to owner actor if TEXTS SHOULD be attached to the owner after spawning.
  (if (`self.AttachToActor`)
    (`self.K2_AttachToActor` (`self.ParentActor`) "None" "KeepRelative" "KeepRelative" "KeepRelative"))
  ;[1 1 1] Kick off a timer that periodically checks if owner is still valid (and destroy self if not)
  (`KismetSystemLibrary.K2_SetTimerDelegate` (`|CreateDelegate` :!event `DestroyIfOwnerInvalid`) (`KismetMathLibrary.RandomFloatInRange` 2.0 3.0) true))

(fn `UserConstructionScript`)